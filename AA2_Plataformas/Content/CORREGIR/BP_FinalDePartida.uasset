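; End-of-game actor that spawns two keys and announces victory when the player enters its door trigger.
; BeginPlay places a BP_Key at each key holder; player overlaps with the two key triggers set their collected flags.
; Entering the door trigger fades out the audio manager's music, plays a victory sound, prints a win message and destroys that trigger.
; The win branch does not check the key flags.
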(event EventBeginPlay
  ;[0.4116 0.8261 1] Al iniciarse, spawnea dos llaves a las dos posiciones específicas de key holders
  (Game|SpawnActorfromClass "/Game/CORREGIR/BP_Key.BP_Key_C" (Math|Conversions|ToTransform(Vector) (Transformation|GetWorldLocation (Variables|Default|Getkey1Holder))) "Undefined" "MultiplyWithRoot" 0 0)
  (Game|SpawnActorfromClass "/Game/CORREGIR/BP_Key.BP_Key_C" (Math|Conversions|ToTransform(Vector) (Transformation|GetWorldLocation (Variables|Default|Getkey2Holder))) "Undefined" "MultiplyWithRoot" 0 0))

(event Collision|EventActorBeginOverlap
  (params (OtherActor :type Actor%20Object%20Reference))
  ;[0.8621 0.4871 1] Si ha colisionado uno de los triggers con el jugador, se inicia una sequencia
  (bind _asbp_third_person_character (Utilities|Casting|CastToBP_ThirdPersonCharacter OtherActor))
  (Utilities|FlowControl|Sequence
    (:then_0
      ;[1 1 1] Si ha colisionado con la primera llave, se asigna que esta recogida
      (if (Collision|IsOverlappingActor (Variables|Default|GetcolTrigger1) _asbp_third_person_character :!class /Script/Engine.PrimitiveComponent)
        (Variables|Default|SetcollectedKey1 true)))
    (:then_1
      ;[1 1 1] Si ha colisionado con la segunda llave, se asigna que esta recogida
      (if (Collision|IsOverlappingActor (Variables|Default|GetcolTrigger2) _asbp_third_person_character :!class /Script/Engine.PrimitiveComponent)
        (Variables|Default|SetcollectedKey2 true)))
    (:then_2
      ;[0.4221 0.446 1] Si ha colisionado con el interior de la puerta, se muestra un mensaje de que has ganado! Finalizando el juego
      (if (Collision|IsOverlappingActor (Variables|Default|Gettrigger) _asbp_third_person_character :!class /Script/Engine.PrimitiveComponent)
        (bind _returnvalue (Actor|GetActorOfClass "/Game/CORREGIR/Audio/BP_AudioManager.BP_AudioManager_C"))
        (Audio|Components|Audio|FadeOut (Variables|/Game/CORREGIR/Audio/BP_AudioManager.BP_AudioManager_C|GetBGMusic _returnvalue) 1.0 0.0 "Linear" :!class /Script/Engine.AudioComponent)
        (Audio|PlaySound2D "/Game/CORREGIR/Audio/MS_Victory2DOneShot.MS_Victory2DOneShot" 1.0 1.0 0.0 0 0)
        (Development|PrintString "YOU WON!" true true "(R=0.000000,G=0.660000,B=1.000000,A=1.000000)" 15.0)
        (Components|DestroyComponent (Variables|Default|Gettrigger))))))

(fn ConstructionScript)