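; BP_MovablePlatform is a platform that moves back and forth between two limits.
; Each Tick offsets the actor along the Arrow component's forward vector by Speed and delta time, without sweep.
; Speed flips sign whenever the platform's Y is at or beyond StartLocation (upper bound) or EndLocation (lower bound).
; The limit check uses only world Y, whatever the arrow's direction, and does not clamp position.
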(event EventTick
  (params (DeltaSeconds :type Float%20%28single-precision%29))
  ;[0.5255 0 0 0.749] La plataforma va hacia la dirección de la flecha * la velocidad
  (Transformation|AddActorWorldOffset (* (* DeltaSeconds (Variables|Default|Getspeed)) (Math|Vector|GetForwardVector (Variables|Default|GetArrow))))
  ;[0.7294 0.02745 0 0.749] Si ha superado uno de los límites puestos de max y min (end, start) entonces la speed se invierte, haciendo que vaya al otro lado
  (if (or (>= (.y (Transformation|GetActorLocation)) (.y (Variables|Default|GetstartLocation))) (>= (.y (Variables|Default|GetendLocation)) (.y (Transformation|GetActorLocation))))
    (Variables|Default|Setspeed (* (Variables|Default|Getspeed) -1.0))))

(fn ConstructionScript)