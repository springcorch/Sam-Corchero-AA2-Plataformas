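; BP_Cannon is a cannon actor that fires BP_Bullet projectiles from four muzzle components on a repeating timer started at BeginPlay.
; Each Shoot call handles the four DirBullet transforms in sequence, tracking one projectile reference per muzzle.
; A still-valid bullet is destroyed without replacement on that call, so a muzzle only spawns when its previous bullet is gone.
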(event Custom|Shoot
  (Utilities|FlowControl|Sequence
    (:then_0
      (Utilities|IsValid (Variables|Default|GetCurrentProjectile)
        (:Is%20Valid
          (Actor|DestroyActor (Variables|Default|GetCurrentProjectile)))
        (:Is%20Not%20Valid
          (bind _returnvalue (Game|SpawnActorfromClass "/Game/CORREGIR/BP_Bullet.BP_Bullet_C" (Transformation|GetWorldTransform (Variables|Default|GetdirBullet)) "Undefined" "MultiplyWithRoot" 0 0))
          (Variables|Default|SetCurrentProjectile _returnvalue))))
    (:then_1
      (Utilities|IsValid (Variables|Default|GetCurrentProjectile1)
        (:Is%20Valid
          (Actor|DestroyActor (Variables|Default|GetCurrentProjectile1)))
        (:Is%20Not%20Valid
          (bind _returnvalue_2 (Game|SpawnActorfromClass "/Game/CORREGIR/BP_Bullet.BP_Bullet_C" (Transformation|GetWorldTransform (Variables|Default|GetdirBullet1)) "Undefined" "MultiplyWithRoot" 0 0))
          (Variables|Default|SetCurrentProjectile1 _returnvalue_2))))
    (:then_2
      (Utilities|IsValid (Variables|Default|GetCurrentProjectile2)
        (:Is%20Valid
          (Actor|DestroyActor (Variables|Default|GetCurrentProjectile2)))
        (:Is%20Not%20Valid
          (bind _returnvalue_3 (Game|SpawnActorfromClass "/Game/CORREGIR/BP_Bullet.BP_Bullet_C" (Transformation|GetWorldTransform (Variables|Default|GetdirBullet2)) "Undefined" "MultiplyWithRoot" 0 0))
          (Variables|Default|SetCurrentProjectile2 _returnvalue_3))))
    (:then_3
      (Utilities|IsValid (Variables|Default|GetCurrentProjectile3)
        (:Is%20Valid
          (Actor|DestroyActor (Variables|Default|GetCurrentProjectile3)))
        (:Is%20Not%20Valid
          (bind _returnvalue_4 (Game|SpawnActorfromClass "/Game/CORREGIR/BP_Bullet.BP_Bullet_C" (Transformation|GetWorldTransform (Variables|Default|GetdirBullet3)) "Undefined" "MultiplyWithRoot" 0 0))
          (Variables|Default|SetCurrentProjectile3 _returnvalue_4))))))

(event EventBeginPlay
  (Utilities|Time|SetTimerbyEvent (delegate Custom|Shoot) 2.5 true))

(fn ConstructionScript)