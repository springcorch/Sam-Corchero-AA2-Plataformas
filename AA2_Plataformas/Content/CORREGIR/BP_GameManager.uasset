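; BP_GameManager runs a timed key-collection challenge that opens the end-of-game door.
; KeyCollected increments the key count and starts a looping one-second TimerSet timer by function name.
; TimerSet prints the countdown from five seconds, stops once two keys are held and rotates the BP_FinalDePartida door.
; If time runs out first, it destroys the third-person character, with no explicit level restart here despite the comment.
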(event EventBeginPlay
  ;[1 0.3995 0.9747] Al iniciar se asigna el timeRemaining a 5
  (Variables|Default|SetTimeRemaining 5))

(fn ConstructionScript)

(fn KeyCollected
  ;[0.9863 0.5125 1] Función que se llama al recolectar una key, sumando las keys recolectadas e iniciando el timer
  (Variables|Default|SetkeysCollected (+ (Variables|Default|GetkeysCollected) 1))
  (if (> (Variables|Default|GetkeysCollected) 0)
    (Utilities|Time|SetTimerbyFunctionName 0 "TimerSet" 1.0 true)))

(fn TimerSet
  ;[1 0.9919 0.5187] Timer que se llama cada un segundo para hacer la cuenta atrás, si se han recolectado las keys necesarias, se para el timer y se abre la puerta -90 grados
  (bind _output_get (Variables|Default|SetTimeRemaining (- (Variables|Default|GetTimeRemaining) 1)))
  (Development|PrintString (Utilities|String|ToString(Integer) _output_get))
  (if (>= (Variables|Default|GetkeysCollected) 2)
    (Utilities|Time|ClearTimerbyFunctionName 0 "TimerSet")
    (Development|PrintString "WELL DONE!" true true "(R=0.000000,G=0.660000,B=1.000000,A=1.000000)" 5.0)
    (bind _returnvalue (Actor|GetActorOfClass "/Game/CORREGIR/BP_FinalDePartida.BP_FinalDePartida_C"))
    (Transformation|AddWorldRotation (Variables|/Game/CORREGIR/BP_FinalDePartida.BP_FinalDePartida_C|Getdoor _returnvalue) (Math|Rotator|MakeRotator 0.0 0.0 -9e+01) true false)
    (else
      ;[0.4086 1 0.6856] Si no se ha llegado a las llaves mínimas y el timer se ha acabado... Se para el timer y se destruye nuestro player, reiniciando el nivel
      (if (== (Variables|Default|GetTimeRemaining) 0)
        (Utilities|Time|ClearTimerbyFunctionName 0 "TimerSet")
        (bind _returnvalue_2 (Actor|GetActorOfClass "/Game/CORREGIR/BP_ThirdPersonCharacter.BP_ThirdPersonCharacter_C"))
        (Actor|DestroyActor _returnvalue_2)
        (Development|PrintString "TIME'S UP!")))))